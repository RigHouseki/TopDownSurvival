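; Base character Blueprint shared by player and enemies, handling damage, death and a player-only dash.
; AnyDamage feeds BPCHealth unless blocked by invincibility, then starts a player grace period or refreshes enemy UI by casting self to BP_Enemy_BASE.
; Death hides the character and spawns BP_EnemyDestruct; non-players also drop a coin and are destroyed.
; Left Shift spends Dash charge on a briefly invincible velocity-based launch, then a looping delay regenerates charge.
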(event `self.ReceiveAnyDamage`
  (params (Damage :type "Float (single-precision)") (DamageType :type "DamageType Object Reference") (InstigatedBy :type "Controller Object Reference") (DamageCauser :type "Actor Object Reference"))
  (bind (_returnvalue_location _returnvalue_rotation _returnvalue_scale) (`KismetMathLibrary.BreakTransform` (`SceneComponent.K2_GetComponentToWorld` (`self.Mesh`))))
  ; AnyDamage
  (if (`self.WasDamaged?`)
    _
    (elif (`self.IsInvincible?`)
      (`KismetSystemLibrary.PrintString` "Dodge")
      (elif (not (`/Game/Blueprints/Components/BPC_Health.IsDefeated` (`self.BPC_Health`)))
        (`/Game/Blueprints/Components/BPC_Health.DecreaseHealth` (`self.BPC_Health`) Damage)
        (`KismetSystemLibrary.PrintString` (`KismetStringLibrary.Conv_DoubleToString` (`/Game/Blueprints/Components/BPC_Health.CurrentHealth` (`self.BPC_Health`))))
        (`KismetSystemLibrary.PrintString` (`KismetStringLibrary.Conv_BoolToString` (`/Game/Blueprints/Components/BPC_Health.IsDefeated` (`self.BPC_Health`))))
        (if (`/Game/Blueprints/Components/BPC_Health.IsDefeated` (`self.BPC_Health`))
          ; Smierc
          (`/Engine/EditorBlueprintResources/StandardMacros.DoOnce` false
            (:`Completed`
              (`|ExecutionSequence`
                (:`then_0`
                  (`ActorComponent.Deactivate` (`self.CharacterMovement`)))
                (:`then_1`
                  (if (`/Game/Blueprints/Components/BPC_Health.IsDefeated` (`self.BPC_Health`))
                    (`SceneComponent.SetHiddenInGame` (`self.Mesh`) true false)
                    (`|SpawnActorFromClass` "/Game/Blueprints/Effects/BP_EnemyDestruct.BP_EnemyDestruct_C" (`KismetMathLibrary.MakeTransform` (- (`self.K2_GetActorLocation`) (0.0 0.0 100.0))) "Undefined" "MultiplyWithRoot" null null)
                    (`self.SetActorHiddenInGame` true)
                    (`self.SetActorEnableCollision` false)
                    (if (not (`self.IsPlayer?`))
                      (`|ExecutionSequence`
                        (:`then_0`
                          (`KismetSystemLibrary.Delay` 0.2)
                          (`self.K2_DestroyActor`))
                        (:`then_1`
                          (`|SpawnActorFromClass` "/Game/Blueprints/Items/Interactibles/Coin/BP_Coin.BP_Coin_C" (`KismetMathLibrary.MakeTransform` (- _returnvalue_location (0.0 0.0 40.0)) _returnvalue_rotation _returnvalue_scale) "Undefined" "MultiplyWithRoot" null null)))))))))
          (elif (`self.IsPlayer?`)
            (`self.IsDamaged?`)
            (else
              ;; jesli enemy, update hp
              (bind _asbp_enemy_base (cast `/Game/Blueprints/Characters/BP_Enemy_BASE` self))
              (`/Game/Blueprints/Characters/BP_Enemy_BASE.UpdateEnemyUI` _asbp_enemy_base))))))))

(event `Key|LeftShift`
  (params (Key :type "Key Structure"))
  (bind (_returnvalue_x _returnvalue_y) (`KismetMathLibrary.BreakVector` (`self.GetVelocity`)))
  (bind (_returnvalue_x_2 _returnvalue_y_2) (`KismetMathLibrary.BreakVector` (* (`KismetMathLibrary.MakeVector` _returnvalue_x _returnvalue_y) 5.0)))
  ;[0.02729 0.15 0.01691 0.5] Dash
  (:`Pressed`
    (if (`self.IsPlayer?`)
      (if (>= (`self.Dash%`) 100.0)
        (if (> (`KismetMathLibrary.VSize` (`CharacterMovementComponent.GetLastUpdateVelocity` (`self.CharacterMovement`))) 0.0)
          (if (not (`self.PlayerDashing`))
            (set `self.PlayerDashing` true)
            (set `self.IsInvincible?` true)
            (`self.LaunchCharacter` (`GameplayStatics.GetPlayerCharacter` 0) (`KismetMathLibrary.MakeVector` _returnvalue_x_2 _returnvalue_y_2) false false)
            (set `self.Dash%` (- (`self.Dash%`) 100.0))
            (`KismetSystemLibrary.Delay` 0.3)
            (set `self.IsInvincible?` false)
            (set `self.PlayerDashing` false)
            ;; Dash Regen speed
            (`KismetSystemLibrary.RetriggerableDelay` 0.2 :!label _label)
            (`self.DashRegen`)
            (goto _label)))))))

(fn `DashRegen`
  ; Dash Regen
  (if (not (== (`self.Dash%`) 100.0))
    (set `self.Dash%` (+ (`self.Dash%`) 10.0))))

(fn `UserConstructionScript`)