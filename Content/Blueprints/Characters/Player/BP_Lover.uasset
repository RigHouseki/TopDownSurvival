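; Player character for a top-down shooter, with aimed movement, spread firing, grenades and placeable barricades, sentry guns and bear traps.
; Enhanced Input and debug keys drive actions, including loot boxes and a pause-based wave shop.
; Tracks XP levels and random pill effects on health, coins or timed speed, pushing updates to the BP_HUD widget.
; Tick writes player position to MPC_Masking for material masking.
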(event Input|EnhancedActionEvents|EnhancedInputActionIA_Move
  (params (ActionValue :type Vector%202D%20Structure) (ElapsedSeconds :type Float%20%28double-precision%29) (TriggeredSeconds :type Float%20%28double-precision%29) (InputAction :type Input%20Action%20Object%20Reference :default "/Game/Inputs/Actions/IA_Move.IA_Move"))
  (bind (_x _y) (Math|Vector2D|BreakVector2D ActionValue))
  ;[0.15 0.15 0.15 0.5] Character Movement
  (Pawn|Input|AddMovementInput "1.000000,0.000000,0.000000" _x false)
  (Pawn|Input|AddMovementInput "0.000000,1.000000,0.000000" _y false))

(event Input|EnhancedActionEvents|EnhancedInputActionIA_Fire
  (params (ActionValue :type Boolean) (ElapsedSeconds :type Float%20%28double-precision%29) (TriggeredSeconds :type Float%20%28double-precision%29) (InputAction :type Input%20Action%20Object%20Reference :default "/Game/Inputs/Actions/IA_Fire.IA_Fire"))
  (bind _returnvalue (Transformation|GetActorTransform))
  (bind _returnvalue_2 (Transformation|GetActorRotation))
  (bind _returnvalue_3 (Transformation|GetActorTransform))
  (bind (_roll _pitch _yaw) (Math|Rotator|BreakRotator _returnvalue_2))
  ;[0.15 0.15 0.15 0.5] Strzelanie pociskiem
  (if (not (Variables|/Game/Blueprints/Components/BPC_Health.BPC_Health_C|GetIsDefeated (Variables|Default|GetBPC_Health)))
    (if (> (Variables|Default|GetProjectileCount) 1)
      (for _index (range 1 (Variables|Default|GetProjectileCount))
        (Game|SpawnActorfromClass "/Game/Blueprints/Items/SentryGun/BP_FriendBullet.BP_FriendBullet_C" (Math|Transform|MakeTransform (+ (Math|Vector|RotateVector (Math|Vector|MakeVector (+ (Variables|Default|GetProjectileOffset) (+ (Variables|Default|GetProjectileCount) 7)) 0.0 0.0) (.rotation _returnvalue)) (.location _returnvalue)) (Math|Rotator|CombineRotators (Math|Rotator|MakeRotator _roll _pitch (+ _yaw (- (/ (* (- (Variables|Default|GetProjectileCount) 1) (Variables|Default|GetSpread)) -2.0) 9.5))) (* (Math|Rotator|MakeRotator 0.0 0.0 (Variables|Default|GetSpread)) _index)) "1.000000,1.000000,1.000000") "Undefined" "MultiplyWithRoot" 0 0))
      (else
        (bind _returnvalue_4 (Game|SpawnActorfromClass "/Game/Blueprints/Items/SentryGun/BP_FriendBullet.BP_FriendBullet_C" (Math|Transform|MakeTransform (+ (Math|Vector|RotateVector (Math|Vector|MakeVector (Variables|Default|GetProjectileOffset) 0.0 0.0) (.rotation _returnvalue_3)) (.location _returnvalue_3)) (.rotation _returnvalue_3) (.scale _returnvalue_3)) "Undefined" "MultiplyWithRoot" 0 0))
        (Variables|/Game/Blueprints/Items/SentryGun/BP_FriendBullet.BP_FriendBullet_C|SetIsFriendBullet _returnvalue_4 true)
        (Audio|PlaySoundatLocation (.OutItem (Utilities|Array|Random (Variables|Default|GetGunshots))) (Transformation|GetActorLocation (Game|Player|GetPlayerPawn 0)) "0, 0, 0" 1.0 1.0 0.0 0 0 0 0)))))

(event Input|EnhancedActionEvents|EnhancedInputActionIA_Shop
  (params (ActionValue :type Boolean) (ElapsedSeconds :type Float%20%28double-precision%29) (TriggeredSeconds :type Float%20%28double-precision%29) (InputAction :type Input%20Action%20Object%20Reference :default "/Game/Inputs/Actions/IA_Shop.IA_Shop"))
  ;[0.15 0.15 0.15 0.5] Otwieranie sklepu [M]
  (if (Game|IsGamePaused)
    (Game|SetGamePaused false)
    (bind _foundwidgets (Widget|GetAllWidgetsOfClass (Variables|Default|GetShopWidget) true))
    (Widget|RemovefromParent _foundwidgets)
    (else
      (Game|SetGamePaused true)
      (if (Variables|Default|GetIsPlayer?)
        (if (not (Variables|/Game/Blueprints/Components/BPC_Health.BPC_Health_C|GetIsDefeated (Variables|Default|GetBPC_Health)))
          (bind _returnvalue (UserInterface|CreateWidget "/Game/Blueprints/Systems/Shop/WB_WaveShop.WB_WaveShop_C"))
          (UserInterface|Viewport|AddtoViewport _returnvalue 0))))))

(event Input|EnhancedActionEvents|EnhancedInputActionIA_LookController
  (params (ActionValue :type Vector%202D%20Structure) (ElapsedSeconds :type Float%20%28double-precision%29) (TriggeredSeconds :type Float%20%28double-precision%29) (InputAction :type Input%20Action%20Object%20Reference :default "/Game/Inputs/Actions/IA_LookController.IA_LookController"))
  (bind _returnvalue (Transformation|GetActorLocation))
  ;[0.15 0.15 0.15 0.5] Rozglądanie sie padem
  ;[0.15 0.15 0.15 0.5] Player rotation based on cursor position
  (Transformation|SetActorRotation (Math|Rotator|FindLookatRotation (Math|Vector|MakeVector (.x _returnvalue) (.y _returnvalue) 0.0) (Math|Vector|MakeVector (.x (stale EventLookat Target)) (.y (stale EventLookat Target)) 0.0))))

(event EventBeginPlay
  (bind _returnvalue (Game|GetPlayerController 0))
  (|CallParentFunction)
  (Variables|/Script/Engine.PlayerController|SetbShowMouseCursor _returnvalue true)
  ;[0.15 0.15 0.15 0.5] Mapping Context
  (Input|AddMappingContext (PlayerController|LocalPlayerSubsystems|GetEnhancedInputLocalPlayerSubsystem _returnvalue) "/Game/Inputs/IMC_TDS.IMC_TDS" 0 "(bIgnoreAllPressedKeysUntilRelease=True,bForceImmediately=False,bNotifyUserSettings=False)")
  ;[0.15 0.15 0.15 0.5] aby potem manipulowac predkoscia gracza na jakis okreslony czas - base speed ustawiamy sobie
  (Variables|Default|SetBaseSpeed (Variables|/Script/Engine.CharacterMovementComponent|GetMaxWalkSpeed (Variables|Character|GetCharacterMovement)))
  ;[0.15 0.15 0.15 0.5] ustawiamy hud ref
  (bind _asbp_hud (Utilities|Casting|CastToBP_HUD (HUD|GetHUD (Game|GetPlayerController 0))))
  (Variables|Default|SetHUDRef (Variables|/Game/Blueprints/HUDandUI/BP_HUD.BP_HUD_C|GetHUD_widget _asbp_hud))
  ;[0.15 0.15 0.15 0.5] ustawiamy startowy level hp itp
  (bind _output_get (Variables|Default|SetLevel 1.0))
  (bind _output_get_2 (Variables|Default|SetXPToNextLevel 1e+02))
  (bind _output_get_3 (Variables|Default|SetCurrentXP 0.0))
  (Utilities|IsValid (Variables|Default|GetHUDRef)
    (:Is%20Valid
      (Default|UpdateXP (Variables|Default|GetHUDRef) _output_get_3 _output_get_2 _output_get))))

(event Collision|EventActorBeginOverlap
  (params (OtherActor :type Actor%20Object%20Reference))
  (|CallParentFunction OtherActor))

(event EventTick
  (params (DeltaSeconds :type Float%20%28single-precision%29))
  (|CallParentFunction DeltaSeconds)
  (Rendering|Material|SetVectorParameterValue "/Game/Materials/MPC_Masking.MPC_Masking" "PlayerPosition" (Math|Conversions|ToLinearColor(Vector) (Transformation|GetActorLocation)) :!class /Script/Engine.KismetMaterialLibrary))

(event EventLookat
  (params (Target :type Vector :default "0, 0, 0"))
  (bind _returnvalue (Transformation|GetActorLocation))
  ;[0.15 0.15 0.15 0.5] Player rotation based on cursor position
  (Transformation|SetActorRotation (Math|Rotator|FindLookatRotation (Math|Vector|MakeVector (.x _returnvalue) (.y _returnvalue) 0.0) (Math|Vector|MakeVector (.x Target) (.y Target) 0.0))))

(event Input|ActionEvents|InputActionSetBarricade
  (params (Key :type Key%20Structure :default "None"))
  ;[0.15 0.15 0.15 0.5] Stawianie barykady
  (:Pressed
    (bind _returnvalue (Game|SpawnActorfromClass "/Game/Blueprints/Items/Barricade/BP_Barricade.BP_Barricade_C" (Math|Transform|MakeTransform (+ (+ (Transformation|GetActorLocation) "0.000000,0.000000,-90.000000") (* (Transformation|GetActorForwardVector) 3e+02)) (Transformation|GetActorRotation)) "DontSpawnIfColliding" "MultiplyWithRoot" 0 0))
    (Actor|SetLifeSpan _returnvalue 5.0)))

(event Input|GamepadEvents|DebugKeyGamepadFaceButtonRight
  (params (Key :type Key%20Structure :default "None") (ActionValue :type Input%20Action%20Value%20Structure))
  ;[0.15 0.15 0.15 0.5] Stawianie barykady
  (:Pressed
    (bind _returnvalue (Game|SpawnActorfromClass "/Game/Blueprints/Items/Barricade/BP_Barricade.BP_Barricade_C" (Math|Transform|MakeTransform (+ (+ (Transformation|GetActorLocation) "0.000000,0.000000,-90.000000") (* (Transformation|GetActorForwardVector) 3e+02)) (Transformation|GetActorRotation)) "DontSpawnIfColliding" "MultiplyWithRoot" 0 0))
    (Actor|SetLifeSpan _returnvalue 5.0)))

(event Input|GamepadEvents|GamepadFaceButtonBottom
  (params (Key :type Key%20Structure :default "None"))
  ;[0.15 0.15 0.15 0.5] Granat [T]
  (:Pressed
    (if (>= (Variables|Default|GetGrenade%20Amount) 1)
      (Variables|Default|SetGrenade%20Amount (- (Variables|Default|GetGrenade%20Amount) 1))
      (Game|SpawnActorfromClass "/Game/Blueprints/Weapons/BP_Grenade.BP_Grenade_C" (Math|Transform|MakeTransform (+ (+ (Transformation|GetActorLocation) "0.000000,0.000000,40.000000") (* (Transformation|GetActorForwardVector) 5e+01)) (Transformation|GetActorRotation)) "AlwaysSpawn" "MultiplyWithRoot" 0 0))))

(event Input|KeyboardEvents|T
  (params (Key :type Key%20Structure :default "None"))
  ;[0.15 0.15 0.15 0.5] Granat [T]
  (:Pressed
    (if (>= (Variables|Default|GetGrenade%20Amount) 1)
      (Variables|Default|SetGrenade%20Amount (- (Variables|Default|GetGrenade%20Amount) 1))
      (Game|SpawnActorfromClass "/Game/Blueprints/Weapons/BP_Grenade.BP_Grenade_C" (Math|Transform|MakeTransform (+ (+ (Transformation|GetActorLocation) "0.000000,0.000000,40.000000") (* (Transformation|GetActorForwardVector) 5e+01)) (Transformation|GetActorRotation)) "AlwaysSpawn" "MultiplyWithRoot" 0 0))))

(event Input|KeyboardEvents|H
  (params (Key :type Key%20Structure :default "None"))
  ;[0.15 0.15 0.15 0.5] Stawianie potrzasku [H]
  (:Pressed
    (Game|SpawnActorfromClass "/Game/Blueprints/Items/BearTrap/BP_BearTrap.BP_BearTrap_C" (Math|Transform|MakeTransform (+ (+ (Transformation|GetActorLocation) "0.000000,0.000000,-80.000000") (* (Transformation|GetActorForwardVector) 1e+02)) (Transformation|GetActorRotation)) "DontSpawnIfColliding" "MultiplyWithRoot" 0 0)))

(event Input|KeyboardEvents|C
  (params (Key :type Key%20Structure :default "None"))
  ;[0.15 0.15 0.15 0.5] piguly
  ;;[0.15 0.15 0.15 0.5] losowe piguly - uzycie
  (:Pressed
    (if (Variables|Default|GetHasPill)
      (CallFunction|RandomPillEffect)
      (Variables|Default|SetHasPill false)
      (CallFunction|HidePillUIPlayer))))

(event Input|GamepadEvents|GamepadFaceButtonLeft
  (params (Key :type Key%20Structure :default "None"))
  ;[0.15 0.15 0.15 0.5] Stawianie wieżyczki
  (:Pressed
    (if (>= (Variables|Default|GetTurret%20Amount) 1)
      (Variables|Default|SetTurret%20Amount (- (Variables|Default|GetTurret%20Amount) 1))
      (bind _returnvalue (Game|SpawnActorfromClass "/Game/Blueprints/Items/SentryGun/BP_SentryGun.BP_SentryGun_C" (Math|Transform|MakeTransform (+ (+ (Transformation|GetActorLocation) "0.000000,0.000000,-80.000000") (* (Transformation|GetActorForwardVector) 3e+02)) (Transformation|GetActorRotation)) "DontSpawnIfColliding" "MultiplyWithRoot" 0 0))
      (Actor|SetLifeSpan _returnvalue 2e+01)
      (else
        (Development|PrintString "NOPE")))))

(event Input|KeyboardEvents|G
  (params (Key :type Key%20Structure :default "None"))
  ;[0.15 0.15 0.15 0.5] Stawianie wieżyczki
  (:Pressed
    (if (>= (Variables|Default|GetTurret%20Amount) 1)
      (Variables|Default|SetTurret%20Amount (- (Variables|Default|GetTurret%20Amount) 1))
      (bind _returnvalue (Game|SpawnActorfromClass "/Game/Blueprints/Items/SentryGun/BP_SentryGun.BP_SentryGun_C" (Math|Transform|MakeTransform (+ (+ (Transformation|GetActorLocation) "0.000000,0.000000,-80.000000") (* (Transformation|GetActorForwardVector) 3e+02)) (Transformation|GetActorRotation)) "DontSpawnIfColliding" "MultiplyWithRoot" 0 0))
      (Actor|SetLifeSpan _returnvalue 2e+01)
      (else
        (Development|PrintString "NOPE")))))

(event Input|KeyboardEvents|E
  (params (Key :type Key%20Structure :default "None"))
  (bind _overlappingactors (Collision|GetOverlappingActors "/Game/Blueprints/Items/Interactibles/LootBox/BP_LootBox.BP_LootBox_C" :!class /Script/Engine.Actor))
  ;[0.15 0.15 0.15 0.5] otwieranie skrzynki
  (:Pressed
    (if (> (Utilities|Array|Length _overlappingactors) 0)
      (Default|OpenChest (Utilities|Array|Get(acopy) _overlappingactors)))))

(event Input|KeyboardEvents|Q
  (params (Key :type Key%20Structure :default "None"))
  ;[0.15 0.15 0.15 0.5] przelaczanie pomocniczego menu
  (:Pressed
    (if (Variables|Default|GetControlsPanelVisible)
      (CallFunction|HideControlsPanel)
      (else
        (CallFunction|ShowControlsPanel)))))

(event Input|GamepadEvents|GamepadLeft2D
  (params (AxisValue :type Vector :default "0, 0, 0"))
  ;[0.15 0.15 0.15 0.5] Zczytywanie danych z lewej gały
)

(fn ConstructionScript
  (|CallParentFunction))

(fn RandomPillEffect
  (bind _bpc_health (Variables|Default|GetBPC_Health))
  (bind _bpc_health_2 (Variables|Default|GetBPC_Health))
  (bind _bpc_health_3 (Variables|Default|GetBPC_Health))
  ;[0.15 0.15 0.15 0.5] losowanie efektu
  (switch int (Math|Random|RandomIntegerinRange 0 4)
    (:0
      (Development|PrintString "HEALTH +20")
      ;[0.15 0.15 0.15 0.5] dodawanie extra hp
      (if (>= (+ (Variables|/Game/Blueprints/Components/BPC_Health.BPC_Health_C|GetCurrentHealth _bpc_health) 2e+01) (Variables|/Game/Blueprints/Components/BPC_Health.BPC_Health_C|GetMaxHealth _bpc_health))
        ;;[0.15 0.15 0.15 0.5] dodajemy extra
        (Variables|/Game/Blueprints/Components/BPC_Health.BPC_Health_C|SetExtraHealth (Variables|Default|GetBPC_Health) (+ (Math|Float|Absolute(Float) (- (Variables|/Game/Blueprints/Components/BPC_Health.BPC_Health_C|GetMaxHealth (Variables|Default|GetBPC_Health)) (+ (Variables|/Game/Blueprints/Components/BPC_Health.BPC_Health_C|GetCurrentHealth (Variables|Default|GetBPC_Health)) 2e+01))) (Variables|/Game/Blueprints/Components/BPC_Health.BPC_Health_C|GetExtraHealth (Variables|Default|GetBPC_Health))))
        ;;[0.15 0.15 0.15 0.5] full zycie
        (Variables|/Game/Blueprints/Components/BPC_Health.BPC_Health_C|SetCurrentHealth _bpc_health_2 (Variables|/Game/Blueprints/Components/BPC_Health.BPC_Health_C|GetMaxHealth _bpc_health_2))
        (else
          ;;[0.15 0.15 0.15 0.5] jak sie miesci w normalnym hp to dodaj
          (Variables|/Game/Blueprints/Components/BPC_Health.BPC_Health_C|SetCurrentHealth (Variables|Default|GetBPC_Health) (+ (Variables|/Game/Blueprints/Components/BPC_Health.BPC_Health_C|GetCurrentHealth (Variables|Default|GetBPC_Health)) 2e+01))))
      (Utilities|FlowControl|Sequence
        (:then_0
          ;;[0.15 0.15 0.15 0.5] zaaktualizuj hud
          (bind _asbp_hud (Utilities|Casting|CastToBP_HUD (HUD|GetHUD (Game|GetPlayerController 0))))
          (Default|UpdateExtraHP (Variables|/Game/Blueprints/HUDandUI/BP_HUD.BP_HUD_C|GetHUD_widget _asbp_hud) (Variables|/Game/Blueprints/Components/BPC_Health.BPC_Health_C|GetExtraHealth _bpc_health_3) (Variables|/Game/Blueprints/Components/BPC_Health.BPC_Health_C|GetMaxExtraHealth _bpc_health_3)))))
    (:1
      (Development|PrintString "COINS + 3")
      (Variables|Default|SetCoins (+ (Variables|Default|GetCoins) 3)))
    (:2
      (Development|PrintString "COINS - 5")
      (Variables|Default|SetCoins (- (Variables|Default|GetCoins) 5)))
    (:3
      (Development|PrintString "SPEED +200 FOR 10S")
      (Utilities|Time|SetTimerbyFunctionName 0 "ResetSpeed" 1e+01)
      (Variables|/Script/Engine.CharacterMovementComponent|SetMaxWalkSpeed (Variables|Character|GetCharacterMovement) (+ (Variables|Default|GetBaseSpeed) 2e+02)))
    (:4
      (Development|PrintString "SPEED -200 FOR 10S")
      (Utilities|Time|SetTimerbyFunctionName 0 "ResetSpeed" 1e+01)
      (Variables|/Script/Engine.CharacterMovementComponent|SetMaxWalkSpeed (Variables|Character|GetCharacterMovement) (- (Variables|Default|GetBaseSpeed) 2e+02)))))

(fn ResetSpeed
  (Variables|/Script/Engine.CharacterMovementComponent|SetMaxWalkSpeed (Variables|Character|GetCharacterMovement) (Variables|Default|GetBaseSpeed))
  (Development|PrintString "RESET SPEED"))

(fn ShowPillUIPlayer
  ;[0.15 0.15 0.15 0.5] pokaz pill - hud dostaje info by pokazac pill
  (bind _asbp_hud (Utilities|Casting|CastToBP_HUD (HUD|GetHUD (Game|GetPlayerController 0))))
  (Default|ShowPillUI (Variables|/Game/Blueprints/HUDandUI/BP_HUD.BP_HUD_C|GetHUD_widget _asbp_hud))
  (Development|PrintString "SHOW PILL"))

(fn HidePillUIPlayer
  (bind _asbp_hud (Utilities|Casting|CastToBP_HUD (HUD|GetHUD (Game|GetPlayerController 0))))
  (Default|HidePillUI (Variables|/Game/Blueprints/HUDandUI/BP_HUD.BP_HUD_C|GetHUD_widget _asbp_hud))
  (Development|PrintString "HIDE PILL"))

(fn ShowControlsPanel
  (bind _asbp_hud (Utilities|Casting|CastToBP_HUD (HUD|GetHUD (Game|GetPlayerController 0))))
  (Default|ShowControlsPanel (Variables|/Game/Blueprints/HUDandUI/BP_HUD.BP_HUD_C|GetHUD_widget _asbp_hud))
  (Variables|Default|SetControlsPanelVisible true))

(fn HideControlsPanel
  (bind _asbp_hud (Utilities|Casting|CastToBP_HUD (HUD|GetHUD (Game|GetPlayerController 0))))
  (Default|HideControlsPanel (Variables|/Game/Blueprints/HUDandUI/BP_HUD.BP_HUD_C|GetHUD_widget _asbp_hud))
  (Variables|Default|SetControlsPanelVisible false))

(fn AddXP
  (params (amount :type Float%20%28double-precision%29))
  (Variables|Default|SetCurrentXP (+ amount (Variables|Default|GetCurrentXP)))
  (if (>= (Variables|Default|GetCurrentXP) (Variables|Default|GetXPToNextLevel))
    (Variables|Default|SetCurrentXP (- (Variables|Default|GetCurrentXP) (Variables|Default|GetXPToNextLevel)))
    (Variables|Default|SetLevel (+ (Variables|Default|GetLevel) 1.0))
    ;[0.15 0.15 0.15 0.5] lvl skalowanie
    (Variables|Default|SetXPToNextLevel (+ (* (Variables|Default|GetLevel) 5e+01) 1e+02)))
  (Default|UpdateXP (Variables|Default|GetHUDRef) (Variables|Default|GetCurrentXP) (Variables|Default|GetXPToNextLevel) (Variables|Default|GetLevel)))