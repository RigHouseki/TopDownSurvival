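; Base enemy character that turns to face the player, walks on request when able to move, and deals contact damage.
; HurtBox overlap runs a very fast looping timer that damages a living player until overlap ends.
; On BeginPlay it scales max health by its spawner's wave after early waves and caches a stats widget for health updates.
; When destroyed, it reports its defeat to the owning spawner.
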(event `self.ReceiveTick`
  (params (DeltaSeconds :type "Float (single-precision)"))
  (bind (_returnvalue_roll _returnvalue_pitch) (`KismetMathLibrary.BreakRotator` (`self.K2_GetActorRotation`)))
  (bind (_returnvalue_roll_2 _returnvalue_pitch_2 _returnvalue_yaw) (`KismetMathLibrary.BreakRotator` (`KismetMathLibrary.FindLookAtRotation` (`self.K2_GetActorLocation`) (`self.K2_GetActorLocation` (`GameplayStatics.GetPlayerPawn` 0)))))
  ; Rotation based on the player
  (`self.K2_SetActorRotation` (`KismetMathLibrary.MakeRotator` _returnvalue_roll _returnvalue_pitch _returnvalue_yaw)))

(event `WalkTowards`
  (params (WorldDirection :type "Vector Structure"))
  ; Walk towards player custom event
  (if (`self.AbleToMove?`)
    (`self.AddMovementInput` WorldDirection)))

(event `self.HurtBox.OnComponentBeginOverlap`
  (params (OverlappedComponent :type "PrimitiveComponent Object Reference") (OtherActor :type "Actor Object Reference") (OtherComp :type "PrimitiveComponent Object Reference") (OtherBodyIndex :type Integer) (bFromSweep :type Boolean) (SweepResult :type "HitResult Structure (by ref)"))
  ; Obecne Apply Damage (zadaje obrażenia graczowi)
  (bind _asbp_player (cast `/Game/Blueprints/Characters/Player/BP_Player` OtherActor))
  (bind _output_get (set `self.Player Ref` _asbp_player))
  (if (> (`/Game/Blueprints/Components/BPC_Health.CurrentHealth` (`/Game/Blueprints/Characters/BP_CharacterBASE.BPC_Health` _output_get)) 0.0)
    (`KismetSystemLibrary.K2_SetTimer` null "Player Take Damage" 0.001 true)))

(event `self.HurtBox.OnComponentEndOverlap`
  (params (OverlappedComponent :type "PrimitiveComponent Object Reference") (OtherActor :type "Actor Object Reference") (OtherComp :type "PrimitiveComponent Object Reference") (OtherBodyIndex :type Integer))
  ; Obecne Apply Damage (zadaje obrażenia graczowi)
  (cast `/Game/Blueprints/Characters/Player/BP_Player` OtherActor)
  (`KismetSystemLibrary.K2_ClearTimer` null "Player Take Damage"))

(event `self.ReceiveDestroyed`
  (`/Game/Blueprints/Systems/BP_SpawnManager.DefeatedEnemy` (`self.OwningSpawner`) self))

(event `self.ReceiveBeginPlay`
  (bind _bpc_health (`self.BPC_Health`))
  (bind _currentwave (`/Game/Blueprints/Systems/BP_SpawnManager.CurrentWave` (`self.OwningSpawner`)))
  ; widget statow enemy
  (`|ExecutionSequence`
    (:`then_0`
      (if (> _currentwave 3)
        (set `/Game/Blueprints/Components/BPC_Health.MaxHealth` (`KismetMathLibrary.Conv_IntToDouble` (`KismetMathLibrary.FCeil` (/ (* (`/Game/Blueprints/Components/BPC_Health.MaxHealth` _bpc_health) _currentwave) 2.0))) _bpc_health)))
    (:`then_1`
      (bind _aswbp_enemy_stats (cast `/Game/Blueprints/HUDandUI/WBP_EnemyStats` (`WidgetComponent.GetUserWidgetObject` (`self.Stats`))))
      (set `self.EnemyStats` _aswbp_enemy_stats))))

(event `UpdateEnemyUI`
  (bind _bpc_health (`self.BPC_Health`))
  ; update zycia enemy przy dmg
  (`/Game/Blueprints/HUDandUI/WBP_EnemyStats.UpdateHealth` (`self.EnemyStats`) (`/Game/Blueprints/Components/BPC_Health.CurrentHealth` _bpc_health) (`/Game/Blueprints/Components/BPC_Health.MaxHealth` _bpc_health)))

(fn `Player Take Damage`
  (bind _player_ref (`self.Player Ref`))
  (if (`PrimitiveComponent.IsOverlappingActor` (`self.HurtBox`) _player_ref)
    (`GameplayStatics.ApplyDamage` _player_ref (`self.Amount`) null self)))

(fn `UserConstructionScript`
  (`parent.UserConstructionScript`))