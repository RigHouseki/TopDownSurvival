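; Shooter enemy that fires bullets at the player when the player is within its gun range.
; A looping one-second timer started on BeginPlay checks EnemyGunRange for an overlapping BP_Player.
; Each hit spawns a BP_EnemyBullet at the enemy's location, rotated toward the first player found.
; The HurtBox overlap event is empty, and the friendly-bullet damage logic is disconnected and never runs.
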(event `self.ReceiveBeginPlay`
  (`parent.ReceiveBeginPlay`)
  (`KismetSystemLibrary.K2_SetTimerDelegate` (delegate `EnemyShot`) 1.0 true))

(event `EnemyShot`
  (bind _returnvalue (`self.K2_GetActorLocation`))
  (bind _overlappingactors (`PrimitiveComponent.GetOverlappingActors` (`self.EnemyGunRange`) "/Game/Blueprints/Characters/Player/BP_Player.BP_Player_C"))
  (if (> (`KismetArrayLibrary.Array_Length` _overlappingactors) 0)
    (`|SpawnActorFromClass` "/Game/Blueprints/Items/SentryGun/BP_EnemyBullet.BP_EnemyBullet_C" (`KismetMathLibrary.MakeTransform` _returnvalue (`KismetMathLibrary.FindLookAtRotation` _returnvalue (`self.K2_GetActorLocation` (`|GetArrayItem` _overlappingactors)))) "AlwaysSpawn" "MultiplyWithRoot" null null)))

(event `self.HurtBox.OnComponentBeginOverlap`
  (params (OverlappedComponent :type "PrimitiveComponent Object Reference") (OtherActor :type "Actor Object Reference") (OtherComp :type "PrimitiveComponent Object Reference") (OtherBodyIndex :type Integer) (bFromSweep :type Boolean) (SweepResult :type "HitResult Structure (by ref)")))

(fn `UserConstructionScript`
  (`parent.UserConstructionScript`))