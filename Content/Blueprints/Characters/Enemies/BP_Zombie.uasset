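; BP_Zombie is an enemy character Blueprint that chases the player.
; On BeginPlay it runs FindPlayer, which, while AbleToMove is set, issues an AI MoveTo toward player character 0.
; Both success and failure of the move call FindPlayer again, so pursuit repeats until AbleToMove is false.
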(event `self.ReceiveBeginPlay`
  (`parent.ReceiveBeginPlay`)
  (`self.FindPlayer`))

(event `FindPlayer`
  (if (`self.AbleToMove?`)
    (`|AIMoveTo` self (0.0 0.0 0.0) (`GameplayStatics.GetPlayerCharacter` 0)
      (:`OnSuccess`
        _)
      (:`OnFail`
        _))
    (`self.FindPlayer`)))

(fn `UserConstructionScript`
  (`parent.UserConstructionScript`))