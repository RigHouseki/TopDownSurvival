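; BP_LootBox is a one-time interactable chest that grants the player a random reward: coins, XP or a pill.
; An interaction sphere toggles a prompt widget and PlayerInRange while the chest is closed.
; OpenChest applies the reward to BP_Player, then shows a WBP_LootPopup projected above the player's head and marks the chest opened.
; Nothing here calls OpenChest, and the old in-file opening logic is disconnected.
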(event `self.ReceiveBeginPlay`
  ; Trzeba bylo dodać żeby działał input E
  (`self.EnableInput` (`GameplayStatics.GetPlayerController` 0))
  (`SceneComponent.SetVisibility` (`self.InteractionWidget`) false false))

(event `Key|Gamepad_FaceButton_Top`
  (params (Key :type "Key Structure"))
  ; Stary system otwierania skrzynki
)

(event `self.InteractionSphere.OnComponentBeginOverlap`
  (params (OverlappedComponent :type "PrimitiveComponent Object Reference") (OtherActor :type "Actor Object Reference") (OtherComp :type "PrimitiveComponent Object Reference") (OtherBodyIndex :type Integer) (bFromSweep :type Boolean) (SweepResult :type "HitResult Structure (by ref)"))
  ; Sprawdzanie czy gracz jest w zasiegu skrzynki / wyswietlanie widgetu "E"
  (if (not (`self.IsOpened`))
    (`SceneComponent.SetVisibility` (`self.InteractionWidget`) true false)
    (set `self.PlayerInRange` true)))

(event `Key|E`
  (params (Key :type "Key Structure"))
  ; Stary system otwierania skrzynki
)

(event `self.InteractionSphere.OnComponentEndOverlap`
  (params (OverlappedComponent :type "PrimitiveComponent Object Reference") (OtherActor :type "Actor Object Reference") (OtherComp :type "PrimitiveComponent Object Reference") (OtherBodyIndex :type Integer))
  ; Sprawdzanie czy gracz jest w zasiegu skrzynki / wyswietlanie widgetu "E"
  (`SceneComponent.SetVisibility` (`self.InteractionWidget`) false false)
  (set `self.PlayerInRange` false))

(fn `OpenChest`
  (if (not (`self.IsOpened`))
    (switch `int` (`KismetMathLibrary.RandomIntegerInRange` 0 2)
      (:`0`
        ; dodawanie coins
        (bind _asbp_player (cast `/Game/Blueprints/Characters/Player/BP_Player` (`GameplayStatics.GetPlayerCharacter` 0)))
        (set `/Game/Blueprints/Characters/Player/BP_Player.Coins` (+ (`/Game/Blueprints/Characters/Player/BP_Player.Coins` _asbp_player) 4) _asbp_player)
        (set `self.LootIcon` "/Game/UI/coin.coin")
        (set `self.LootText` "+4")
        (`KismetSystemLibrary.PrintString` "DODANIE COINS ZE SKRZYNKI"))
      (:`1`
        ; dodawanie xp
        (bind _asbp_player_2 (cast `/Game/Blueprints/Characters/Player/BP_Player` (`GameplayStatics.GetPlayerCharacter` 0)))
        (`/Game/Blueprints/Characters/Player/BP_Player.AddXP` _asbp_player_2 100.0)
        (set `self.LootIcon` "/Game/UI/xp_icon.xp_icon")
        (set `self.LootText` "+100")
        (`KismetSystemLibrary.PrintString` "DODANIE XP ZE SKRZYNKI"))
      (:`2`
        ; dodawanie piguły
        (bind _asbp_player_3 (cast `/Game/Blueprints/Characters/Player/BP_Player` (`GameplayStatics.GetPlayerCharacter` 0)))
        (set `/Game/Blueprints/Characters/Player/BP_Player.HasPill` true _asbp_player_3)
        (`/Game/Blueprints/Characters/Player/BP_Player.ShowPillUI_player` _asbp_player_3)
        (set `self.LootIcon` "/Game/UI/pill.pill")
        (set `self.LootText` "+")
        (`KismetSystemLibrary.PrintString` "DODANIE PILL ZE SKRZYNKI")))
    (bind _returnvalue (`|CreateWidget` "/Game/Blueprints/HUDandUI/WBP_LootPopup.WBP_LootPopup_C" (`GameplayStatics.GetPlayerController` 0)))
    (bind _output_get (set `self.LootPopupRef` _returnvalue))
    (`/Game/Blueprints/HUDandUI/WBP_LootPopup.InitLoot` _output_get (`self.LootIcon`) (`self.LootText`))
    (`UserWidget.AddToViewport` _output_get 0)
    (`UserWidget.SetPositionInViewport` _output_get (`GameplayStatics.ProjectWorldToScreen` (`GameplayStatics.GetPlayerController` 0) (+ (`self.K2_GetActorLocation` (`GameplayStatics.GetPlayerCharacter` 0)) (0.0 0.0 100.0))) true)
    (set `self.IsOpened` true)
    (`SceneComponent.SetVisibility` (`self.InteractionWidget`) false false)))

(fn `UserConstructionScript`)