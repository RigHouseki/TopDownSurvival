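; Friendly projectile for the sentry gun that damages actors tagged Enemy and expires after a two-second lifespan.
; It caches the player on BeginPlay and uses the player's DamageAmount for damage.
; A blocking hit applies damage once through DoOnce, prints a debug string, then destroys the bullet after a short delay.
; The Hitbox separately applies damage on overlap begin and destroys the bullet on overlap end.
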(event `self.ReceiveBeginPlay`
  (`parent.ReceiveBeginPlay`)
  (`|ExecutionSequence`
    (:`then_0`
      (bind _asbp_player (cast `/Game/Blueprints/Characters/Player/BP_Player` (`GameplayStatics.GetPlayerCharacter` 0)))
      (set `self.Player Ref` _asbp_player))
    (:`then_1`
      (`self.SetLifeSpan` 2.0))))

(event `self.ReceiveHit`
  (params (MyComp :type "PrimitiveComponent Object Reference") (Other :type "Actor Object Reference") (OtherComp :type "PrimitiveComponent Object Reference") (bSelfMoved :type Boolean) (HitLocation :type "Vector Structure") (HitNormal :type "Vector Structure") (NormalImpulse :type "Vector Structure") (Hit :type "HitResult Structure (by ref)"))
  (if (`self.ActorHasTag` Other "Enemy")
    (`|ExecutionSequence`
      (:`then_0`
        (`/Engine/EditorBlueprintResources/StandardMacros.DoOnce` false
          (:`Completed`
            (`GameplayStatics.ApplyDamage` Other (`/Game/Blueprints/Characters/BP_CharacterBASE.DamageAmount` (`self.Player Ref`)) null self)
            (`KismetSystemLibrary.PrintString` "Ouch"))))
      (:`then_1`
        (`KismetSystemLibrary.Delay` 0.05)
        (`self.K2_DestroyActor`)))
    (elif (`self.ActorHasTag` Other "Player")
      _)))

(event `self.hitbox.OnComponentBeginOverlap`
  (params (OverlappedComponent :type "PrimitiveComponent Object Reference") (OtherActor :type "Actor Object Reference") (OtherComp :type "PrimitiveComponent Object Reference") (OtherBodyIndex :type Integer) (bFromSweep :type Boolean) (SweepResult :type "HitResult Structure (by ref)"))
  (if (`self.ActorHasTag` OtherActor "Enemy")
    (`GameplayStatics.ApplyDamage` OtherActor (`/Game/Blueprints/Characters/BP_CharacterBASE.DamageAmount` (`self.Player Ref`)) null self)))

(event `self.hitbox.OnComponentEndOverlap`
  (params (OverlappedComponent :type "PrimitiveComponent Object Reference") (OtherActor :type "Actor Object Reference") (OtherComp :type "PrimitiveComponent Object Reference") (OtherBodyIndex :type Integer))
  (if (`self.ActorHasTag` OtherActor "Enemy")
    (`self.K2_DestroyActor`)))

(fn `UserConstructionScript`
  (`parent.UserConstructionScript`))