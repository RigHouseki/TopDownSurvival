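; Enemy bullet projectile from the sentry gun item set that damages the player and expires after a short lifespan.
; A hit on a Player-tagged actor deals fixed damage once, then destroys the bullet after a brief delay.
; A separate Box overlap applies BulletDamage to any BP_Player that is not the owner, without destroying the bullet.
; BeginPlay caches a player reference that these graphs never read.
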(event `self.ReceiveBeginPlay`
  (`parent.ReceiveBeginPlay`)
  (`|ExecutionSequence`
    (:`then_0`
      (bind _asbp_player (cast `/Game/Blueprints/Characters/Player/BP_Player` (`GameplayStatics.GetPlayerCharacter` 0)))
      (set `self.Player Ref` _asbp_player))
    (:`then_1`
      (`self.SetLifeSpan` 2.0))))

(event `self.ReceiveHit`
  (params (MyComp :type "PrimitiveComponent Object Reference") (Other :type "Actor Object Reference") (OtherComp :type "PrimitiveComponent Object Reference") (bSelfMoved :type Boolean) (HitLocation :type "Vector Structure") (HitNormal :type "Vector Structure") (NormalImpulse :type "Vector Structure") (Hit :type "HitResult Structure (by ref)"))
  (if (`self.ActorHasTag` Other "Player")
    (`|ExecutionSequence`
      (:`then_0`
        (`/Engine/EditorBlueprintResources/StandardMacros.DoOnce` false
          (:`Completed`
            (`GameplayStatics.ApplyDamage` Other 5.0)
            (`KismetSystemLibrary.PrintString` "Player Strike"))))
      (:`then_1`
        (`KismetSystemLibrary.Delay` 0.05)
        (`self.K2_DestroyActor`)))
    (else
      (`KismetSystemLibrary.PrintString` "bwaaah?"))))

(event `self.Box.OnComponentBeginOverlap`
  (params (OverlappedComponent :type "PrimitiveComponent Object Reference") (OtherActor :type "Actor Object Reference") (OtherComp :type "PrimitiveComponent Object Reference") (OtherBodyIndex :type Integer) (bFromSweep :type Boolean) (SweepResult :type "HitResult Structure (by ref)"))
  (bind _asbp_player (cast `/Game/Blueprints/Characters/Player/BP_Player` OtherActor))
  (if (!= _asbp_player (`self.GetOwner`))
    (`GameplayStatics.ApplyDamage` OtherActor (`self.BulletDamage`) null self)))

(fn `UserConstructionScript`
  (`parent.UserConstructionScript`))