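; BP_SentryGun is a stationary turret that shoots at the player while they are within range.
; Overlap events on the SentryGunRange component set an in-range flag when a BP_Player enters or leaves.
; A looping one-second timer started on BeginPlay checks that flag and spawns a BP_Bullet at the gun's location, rotated toward player 0's current position.
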(event `self.ReceiveBeginPlay`
  (`KismetSystemLibrary.K2_SetTimerDelegate` (delegate `SentryShot`) 1.0 true))

(event `SentryShot`
  (bind _returnvalue (`self.K2_GetActorLocation`))
  (if (`self.InSentryGunRange`)
    (`|SpawnActorFromClass` "/Game/Blueprints/Items/SentryGun/BP_Bullet.BP_Bullet_C" (`KismetMathLibrary.MakeTransform` _returnvalue (`KismetMathLibrary.FindLookAtRotation` _returnvalue (`self.K2_GetActorLocation` (`GameplayStatics.GetPlayerCharacter` 0)))) "AlwaysSpawn" "MultiplyWithRoot" null null)))

(event `self.SentryGunRange.OnComponentBeginOverlap`
  (params (OverlappedComponent :type "PrimitiveComponent Object Reference") (OtherActor :type "Actor Object Reference") (OtherComp :type "PrimitiveComponent Object Reference") (OtherBodyIndex :type Integer) (bFromSweep :type Boolean) (SweepResult :type "HitResult Structure (by ref)"))
  (cast `/Game/Blueprints/Characters/Player/BP_Player` OtherActor)
  (set `self.InSentryGunRange` true))

(event `self.SentryGunRange.OnComponentEndOverlap`
  (params (OverlappedComponent :type "PrimitiveComponent Object Reference") (OtherActor :type "Actor Object Reference") (OtherComp :type "PrimitiveComponent Object Reference") (OtherBodyIndex :type Integer))
  (cast `/Game/Blueprints/Characters/Player/BP_Player` OtherActor)
  (set `self.InSentryGunRange` false))

(fn `UserConstructionScript`)