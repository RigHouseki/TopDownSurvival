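; Bear trap item that is meant to halt a zombie entering its sphere for a few seconds, then destroy itself.
; On overlap it checks for BP_Zombie, then casts that same actor, not its controller, to AIC_Enemy, continuing only if that succeeds.
; It then stops movement, waits, calls WalkTowards toward the target player and destroys itself.
; Other actors only print a debug string; a MaxWalkSpeed change is left unconnected.
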(event `self.Sphere.OnComponentBeginOverlap`
  (params (OverlappedComponent :type "PrimitiveComponent Object Reference") (OtherActor :type "Actor Object Reference") (OtherComp :type "PrimitiveComponent Object Reference") (OtherBodyIndex :type Integer) (bFromSweep :type Boolean) (SweepResult :type "HitResult Structure (by ref)"))
  (cast `/Game/Blueprints/Characters/Enemies/BP_Zombie` OtherActor
    (:`then`
      (bind _asaic_enemy (cast `/Game/AI/AIC_Enemy` OtherActor))
      (`Controller.StopMovement` _asaic_enemy)
      (`KismetSystemLibrary.Delay` 5.0)
      (`/Game/Blueprints/Characters/BP_Enemy_BASE.WalkTowards` (`self.Possessed Pawn`) (`KismetMathLibrary.GetForwardVector` (`KismetMathLibrary.FindLookAtRotation` (`self.K2_GetActorLocation` (`self.Possessed Pawn`)) (`self.K2_GetActorLocation` (`self.TargetPlayer`)))))
      (`self.K2_DestroyActor`))
    (:`CastFailed`
      (`KismetSystemLibrary.PrintString` "nothing"))))

(fn `UserConstructionScript`)