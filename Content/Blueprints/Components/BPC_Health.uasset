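; BPC_Health is a health component that tracks damage and defeat, with comments indicating use by both player and enemies.
; CurrentHealth starts at MaxHealth on BeginPlay.
; DecreaseHealth drains an ExtraHealth buffer first and passes any overflow to CurrentHealth, which is clamped at zero only when no buffer was present.
; It then sets IsDefeated when CurrentHealth is zero or below.
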(event `self.ReceiveBeginPlay`
  (set `self.CurrentHealth` (`self.MaxHealth`)))

(fn `DecreaseHealth`
  (params (IncomingDamage :type "Float (double-precision)"))
  ; gracz
  (if (> (`self.ExtraHealth`) 0.0)
    (if (> (`self.ExtraHealth`) IncomingDamage)
      ;; wystarczajaco extra health
      (set `self.ExtraHealth` (- (`self.ExtraHealth`) IncomingDamage))
      (else
        ;; przy zbyt malej ilosci extra health
        (set `self.CurrentHealth` (- (`self.CurrentHealth`) (`KismetMathLibrary.Abs` (- (`self.ExtraHealth`) IncomingDamage))))
        (set `self.ExtraHealth` 0.0)))
    (else
      ;; enemy
      (set `self.CurrentHealth` (`KismetMathLibrary.FMax` (- (`self.CurrentHealth`) IncomingDamage)))))
  (set `self.IsDefeated` (<= (`self.CurrentHealth`) 0.0)))