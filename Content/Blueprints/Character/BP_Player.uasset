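; Player character for what appears to be a top-down game, with Enhanced Input movement along world axes and a visible mouse cursor.
; A Lookat event rotates the actor toward a supplied target; controller look input enters the same rotation node, but its stick-offset math is unconnected.
; SetBarricade or a gamepad debug key spawns a short-lived BP_Barricade ahead of the player unless blocked.
; Left-stick values print to screen for debugging.
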(event Input|EnhancedActionEvents|EnhancedInputActionIA_Move
  (params (ActionValue :type Vector%202D%20Structure) (ElapsedSeconds :type Float%20%28double-precision%29) (TriggeredSeconds :type Float%20%28double-precision%29) (InputAction :type Input%20Action%20Object%20Reference :default "/Game/Inputs/Actions/IA_Move.IA_Move"))
  (bind (_x _y) (Math|Vector2D|BreakVector2D ActionValue))
  ;[0.15 0.15 0.15 0.5] Character Movement
  (Pawn|Input|AddMovementInput "1.000000,0.000000,0.000000" _x false)
  (Pawn|Input|AddMovementInput "0.000000,1.000000,0.000000" _y false))

(event Input|EnhancedActionEvents|EnhancedInputActionIA_LookController
  (params (ActionValue :type Vector%202D%20Structure) (ElapsedSeconds :type Float%20%28double-precision%29) (TriggeredSeconds :type Float%20%28double-precision%29) (InputAction :type Input%20Action%20Object%20Reference :default "/Game/Inputs/Actions/IA_LookController.IA_LookController"))
  (bind _returnvalue (Transformation|GetActorLocation))
  ;[0.15 0.15 0.15 0.5] Rozglądanie sie padem
  ;[0.15 0.15 0.15 0.5] Player rotation based on cursor position
  (Transformation|SetActorRotation (Math|Rotator|FindLookatRotation (Math|Vector|MakeVector (.x _returnvalue) (.y _returnvalue) 0.0) (Math|Vector|MakeVector (.x (stale EventLookat Target)) (.y (stale EventLookat Target)) 0.0))))

(event EventBeginPlay
  (bind _returnvalue (Game|GetPlayerController 0))
  (|CallParentFunction)
  (Variables|/Script/Engine.PlayerController|SetbShowMouseCursor _returnvalue true)
  ;[0.15 0.15 0.15 0.5] Mapping Context
  (Input|AddMappingContext (PlayerController|LocalPlayerSubsystems|GetEnhancedInputLocalPlayerSubsystem _returnvalue) "/Game/Inputs/IMC_TDS.IMC_TDS" 0 "(bIgnoreAllPressedKeysUntilRelease=True,bForceImmediately=False,bNotifyUserSettings=False)"))

(event Collision|EventActorBeginOverlap
  (params (OtherActor :type Actor%20Object%20Reference))
  (|CallParentFunction OtherActor) ; This node is disabled and will not be called.\nDrag off pins to build functionality.
)

(event EventLookat
  (params (Target :type Vector :default "0, 0, 0"))
  (bind _returnvalue (Transformation|GetActorLocation))
  ;[0.15 0.15 0.15 0.5] Player rotation based on cursor position
  (Transformation|SetActorRotation (Math|Rotator|FindLookatRotation (Math|Vector|MakeVector (.x _returnvalue) (.y _returnvalue) 0.0) (Math|Vector|MakeVector (.x Target) (.y Target) 0.0))))

(event Input|ActionEvents|InputActionSetBarricade
  (params (Key :type Key%20Structure))
  ;[0.15 0.15 0.15 0.5] Stawianie barykady
  (:Pressed
    (bind _returnvalue (Game|SpawnActorfromClass "/Game/Blueprints/Interactibles/Barykada/BP_Barricade.BP_Barricade_C" (Math|Transform|MakeTransform (+ (+ (Transformation|GetActorLocation) "0.000000,0.000000,-90.000000") (* (Transformation|GetActorForwardVector) 3e+02)) (Transformation|GetActorRotation)) "DontSpawnIfColliding" "MultiplyWithRoot" 0 0))
    (Actor|SetLifeSpan _returnvalue 5.0)))

(event Input|GamepadEvents|DebugKeyGamepadFaceButtonRight
  (params (Key :type Key%20Structure) (ActionValue :type Input%20Action%20Value%20Structure))
  ;[0.15 0.15 0.15 0.5] Stawianie barykady
  (:Pressed
    (bind _returnvalue (Game|SpawnActorfromClass "/Game/Blueprints/Interactibles/Barykada/BP_Barricade.BP_Barricade_C" (Math|Transform|MakeTransform (+ (+ (Transformation|GetActorLocation) "0.000000,0.000000,-90.000000") (* (Transformation|GetActorForwardVector) 3e+02)) (Transformation|GetActorRotation)) "DontSpawnIfColliding" "MultiplyWithRoot" 0 0))
    (Actor|SetLifeSpan _returnvalue 5.0)))

(event Input|GamepadEvents|GamepadLeft2D
  (params (AxisValue :type Vector :default "0, 0, 0"))
  ;[0.15 0.15 0.15 0.5] Zczytywanie danych z lewej gały
  (Development|PrintString (Utilities|String|ToString(Vector) AxisValue) true true "(R=0.000000,G=0.660000,B=1.000000,A=1.000000)" 0.1))

(fn ConstructionScript
  (|CallParentFunction))