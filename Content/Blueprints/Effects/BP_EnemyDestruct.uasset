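; BP_EnemyDestruct is the destruction effect for a defeated enemy: a geometry collection that bursts apart, fades out and removes itself.
; On BeginPlay it applies a radial impulse at ImpulseLocation, then shortly afterwards puts a red dynamic material on the collection.
; After a further delay, a looping timer lowers FadeValue into the material's opacity mask parameter for a noise-based dissolve, destroying the actor at the end.
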(event `self.ReceiveBeginPlay`
  (`|ExecutionSequence`
    (:`then_0`
      (`PrimitiveComponent.AddRadialImpulse` (`self.GeometryCollection`) (`SceneComponent.K2_GetComponentLocation` (`self.ImpulseLocation`)) 250.0 500.0 "RIF_Constant" true))
    (:`then_1`
      (`KismetSystemLibrary.Delay` 0.1)
      (bind _returnvalue (`PrimitiveComponent.CreateDynamicMaterialInstance` (`self.GeometryCollection`) 0 "/Game/Materials/M_ColorRed.M_ColorRed" "None"))
      (set `self.DynMaterial` _returnvalue)
      (`KismetSystemLibrary.Delay` 0.7)
      ; zanikanie truchla przeciwnika, co TIME odejmuje fade value, fade value zmienia sie w materiale i odejmowane jest od szumu (by sprawić by material znikal)
      (set `self.FadeValue` 3.0)
      (`KismetSystemLibrary.K2_SetTimerDelegate` (delegate `FadeStep`) 0.05 true))))

(event `FadeStep`
  ; zanikanie truchla przeciwnika, co TIME odejmuje fade value, fade value zmienia sie w materiale i odejmowane jest od szumu (by sprawić by material znikal)
  (bind _output_get (set `self.FadeValue` (- (`self.FadeValue`) 0.1)))
  (if (<= _output_get -1.0)
    (`self.K2_DestroyActor`)
    (else
      (`MaterialInstanceDynamic.SetScalarParameterValue` (`self.DynMaterial`) "OpacityMaskParam" _output_get))))

(fn `UserConstructionScript`)