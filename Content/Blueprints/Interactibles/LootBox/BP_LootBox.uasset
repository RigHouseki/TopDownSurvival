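; BP_LootBox is an interactable loot box that shows an "E" prompt widget while something overlaps its interaction sphere.
; Sphere begin and end overlap toggle the widget and a PlayerInRange flag, with no check on which actor overlaps.
; The actor enables input from player controller 0, so E or the gamepad top face button triggers opening.
; Opening currently only prints a debug string.
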(event `self.ReceiveBeginPlay`
  ; Trzeba bylo dodać żeby działał input E
  (`self.EnableInput` (`GameplayStatics.GetPlayerController` 0))
  (`SceneComponent.SetVisibility` (`self.InteractionWidget`) false false))

(event `self.InteractionSphere.OnComponentBeginOverlap`
  (params (OverlappedComponent :type "PrimitiveComponent Object Reference") (OtherActor :type "Actor Object Reference") (OtherComp :type "PrimitiveComponent Object Reference") (OtherBodyIndex :type Integer) (bFromSweep :type Boolean) (SweepResult :type "HitResult Structure (by ref)"))
  ; Sprawdzanie czy gracz jest w zasiegu skrzynki / wyswietlanie widgetu "E"
  (`SceneComponent.SetVisibility` (`self.InteractionWidget`) true false)
  (set `self.PlayerInRange` true))

(event `Key|Gamepad_FaceButton_Top`
  (params (Key :type "Key Structure"))
  ; E / trójkąt zeby otworzyc skrzynke
  (:`Pressed`
    (if (`self.PlayerInRange`) :!label _label
      (`KismetSystemLibrary.PrintString` "Otwieranie skrzynki"))))

(event `Key|E`
  (params (Key :type "Key Structure"))
  ; E / trójkąt zeby otworzyc skrzynke
  (:`Pressed`
    (goto _label)))

(event `self.InteractionSphere.OnComponentEndOverlap`
  (params (OverlappedComponent :type "PrimitiveComponent Object Reference") (OtherActor :type "Actor Object Reference") (OtherComp :type "PrimitiveComponent Object Reference") (OtherBodyIndex :type Integer))
  ; Sprawdzanie czy gracz jest w zasiegu skrzynki / wyswietlanie widgetu "E"
  (`SceneComponent.SetVisibility` (`self.InteractionWidget`) false false)
  (set `self.PlayerInRange` false))

(fn `UserConstructionScript`)