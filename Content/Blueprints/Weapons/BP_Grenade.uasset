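; BP_Grenade is a grenade projectile actor that freezes shortly after impact and then removes itself, with no explosion or damage logic in this graph.
; The first GrenadeCollicion hit passes a DoOnce, then after a short delay halts ProjectileMovement, zeroes its gravity and turns off physics simulation on its collision and sphere components.
; It prints a debug string during the stop and destroys the actor after a further delay.
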(event `self.GrenadeCollicion.OnComponentHit`
  (params (HitComponent :type "PrimitiveComponent Object Reference") (OtherActor :type "Actor Object Reference") (OtherComp :type "PrimitiveComponent Object Reference") (NormalImpulse :type "Vector Structure") (Hit :type "HitResult Structure (by ref)"))
  (`/Engine/EditorBlueprintResources/StandardMacros.DoOnce` false
    (:`Completed`
      (`KismetSystemLibrary.Delay` 0.2)
      (`ProjectileMovementComponent.SetVelocityInLocalSpace` (`self.ProjectileMovement`) (0.0 0.0 0.0))
      (set `ProjectileMovementComponent.ProjectileGravityScale` 0.0 (`self.ProjectileMovement`))
      (`KismetSystemLibrary.PrintString` "ahaaaaa")
      (`MovementComponent.StopMovementImmediately` (`self.ProjectileMovement`))
      (`PrimitiveComponent.SetSimulatePhysics` (`MovementComponent.UpdatedPrimitive` (`self.ProjectileMovement`)) false)
      (`PrimitiveComponent.SetSimulatePhysics` (`self.GrenadeCollicion`) false)
      (`PrimitiveComponent.SetSimulatePhysics` (`self.Sphere`) false)
      (`KismetSystemLibrary.Delay` 1.0)
      (`self.K2_DestroyActor`))))

(fn `UserConstructionScript`)